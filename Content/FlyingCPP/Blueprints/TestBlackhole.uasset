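; Test black hole actor that pulls physics-simulating pawns toward its center and expires after a set lifetime.
; On BeginPlay it matches the collision sphere's scale to the scene root, and actor overlaps add or remove pawns from an affected list.
; Each tick adds velocity toward the sphere center to each listed pawn's root, strengthening linearly with proximity, without delta-time scaling.
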(event EventBeginPlay
  (Transformation|SetWorldScale3D (Variables|Default|GetSphereCollision) (Transformation|GetWorldScale (Variables|Default|GetDefaultSceneRoot)))
  (Actor|SetLifeSpan (Variables|Default|GetLifeTime)))

(event Collision|EventActorBeginOverlap
  (params (OtherActor :type Actor%20Object%20Reference))
  (bind _aspawn (Utilities|Casting|CastToPawn OtherActor))
  (if (Physics|IsSimulatingPhysics (VehicleSound|GetRootComponent _aspawn) "None")
    (Utilities|Array|AddUnique (Variables|Default|GetAffectedActors) _aspawn)
    (Development|PrintText (Utilities|Text|FormatText "Added {0}" (Utilities|Text|ToText(String) (Utilities|GetObjectName _aspawn))))))

(event EventTick
  (params (DeltaSeconds :type Float%20%28single-precision%29))
  (bind _spherecollision (Variables|Default|GetSphereCollision))
  (bind _returnvalue (Transformation|GetWorldLocation _spherecollision))
  (for _array_element (Variables|Default|GetAffectedActors)
    (bind _asprimitive_component (Utilities|Casting|CastToPrimitiveComponent (VehicleSound|GetRootComponent _array_element)))
    (Physics|SetPhysicsLinearVelocity _asprimitive_component (* (Math|Vector|GetForwardVector (Math|Rotator|FindLookatRotation (Transformation|GetWorldLocation (VehicleSound|GetRootComponent _array_element)) _returnvalue)) (* (Variables|Default|GetMagnitude) (- 1.0 (/ (Math|Vector|VectorLength (- (Transformation|GetWorldLocation (VehicleSound|GetRootComponent _array_element)) _returnvalue)) (Components|Sphere|GetScaledSphereRadius (Variables|Default|GetSphereCollision)))))) true "None")))

(event Collision|EventActorEndOverlap
  (params (OtherActor :type Actor%20Object%20Reference))
  (Utilities|Array|RemoveItem (Variables|Default|GetAffectedActors) OtherActor)
  (Development|PrintText (Utilities|Text|FormatText "Removed {0}" (Utilities|Text|ToText(String) (Utilities|GetObjectName OtherActor)))))

(fn ConstructionScript)