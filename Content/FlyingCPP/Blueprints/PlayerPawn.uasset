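; Player pawn Blueprint that adds input-manager mode toggling and debug feedback to the player's pawn.
; The M key switches the WM input manager between Off and Assign, showing the mouse cursor while assigning and hiding it when off.
; Every tick a debug sphere snaps to the shoot-from point's location and rotation.
; Overlap and hit events print the other actor's name; a shoot-point printout is left unconnected.
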(event EventBeginPlay)

(event EventTick
  (params (DeltaSeconds :type Float%20%28single-precision%29))
  (bind (_location _rotation) (Class|SpaceShooterPawn|GetShootfromPoint))
  (bind _debugsphere (Variables|Default|GetDebugSphere))
  (Transformation|SetWorldRotation _debugsphere _rotation false true)
  (Transformation|SetWorldLocation _debugsphere _location false true))

(event Collision|EventActorBeginOverlap
  (params (OtherActor :type Actor%20Object%20Reference))
  (Development|PrintText (Utilities|Text|FormatText "Started overlapping actor: {0}" (Utilities|Text|ToText(String) (Utilities|GetDisplayName OtherActor)))))

(event Collision|EventHit
  (params (MyComp :type Primitive%20Component%20Object%20Reference) (Other :type Actor%20Object%20Reference) (OtherComp :type Primitive%20Component%20Object%20Reference) (bSelfMoved :type Boolean) (HitLocation :type Vector :default "0, 0, 0") (HitNormal :type Vector :default "0, 0, 0") (NormalImpulse :type Vector :default "0, 0, 0") (Hit :type Hit%20Result%20Structure%20%28by%20ref%29))
  (Development|PrintText (Utilities|Text|FormatText "Hit by actor: {0}" (Utilities|Text|ToText(String) (Utilities|GetDisplayName Other)))))

(event Input|KeyboardEvents|M
  (params (Key :type Key%20Structure :default "AnyKey"))
  (bind _returnvalue (Class|WMControllerFunctionLib|GetWMInputManager))
  (bind _self self)
  (bind _returnvalue_2 (Pawn|GetController _self))
  (:Pressed
    (if (Utilities|Enum|Equal(Enum) (Variables|/Script/WM_InputManager_Plugin.WM_InputManagerBase|GetManagerModeEnum _returnvalue) "off")
      (Class|WMInputManagerBase|SwitchManagerModeEnum _returnvalue "Assign")
      (bind _asplayer_controller (Utilities|Casting|CastToPlayerController _returnvalue_2))
      (Variables|/Script/Engine.PlayerController|SetbShowMouseCursor _asplayer_controller true)
      (else
        (Class|WMInputManagerBase|SwitchManagerModeEnum _returnvalue "off")
        (bind _asplayer_controller_2 (Utilities|Casting|CastToPlayerController _returnvalue_2))
        (Variables|/Script/Engine.PlayerController|SetbShowMouseCursor _asplayer_controller_2 false)))))

(fn ConstructionScript)