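; TestProjectile is a test projectile that spawns a black hole where it explodes.
; It activates its particle component on BeginPlay.
; Its OnExploded event spawns a scaled-up TestBlackhole at the impact location with a set magnitude and lifetime, passing on owner and instigator, then prints the hit actor's name if that actor is valid.
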(event EventBeginPlay
  (Components|Activation|Activate (Variables|Default|GetParticleComp) false))

(event Collision|EventActorBeginOverlap
  (params (OtherActor :type Actor%20Object%20Reference)))

(event EventTick
  (params (DeltaSeconds :type Float%20%28single-precision%29)))

(event EventOnExploded
  (params (ImpactLocation :type Vector%20%28by%20ref%29) (HitActor :type Actor%20Object%20Reference))
  (Game|SpawnActorfromClass "/Game/FlyingCPP/Blueprints/TestBlackhole.TestBlackhole_C" (Math|Transform|MakeTransform ImpactLocation "0, 0, 0" "5.000000,5.000000,5.000000") "AlwaysSpawn" (Components|GetOwner) 2e+02 5.0 (Game|GetInstigator))
  (Utilities|IsValid HitActor
    (:Is%20Valid
      (Development|PrintText (Utilities|Text|FormatText "TestProjectile hit {0}" (Utilities|Text|ToText(String) (Utilities|GetDisplayName HitActor)))))))

(fn ConstructionScript)