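; BP_DynamicGravityForce is a placeable gravity source actor that sets up its visual body and gravity center.
; The construction script applies the configured mesh, material and world scale to the Mesh component.
; It then moves the GravityCenterLocation component to the GravityCenter offset and caches that component's world position in GravityLocation.
; The file contains only this setup, with no logic that applies a force.
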(fn ConstructionScript
  (bind _mesh (Variables|Default|GetMesh))
  (bind _gravitycenterlocation (Variables|Default|GetGravityCenterLocation))
  (Components|StaticMesh|SetStaticMesh _mesh (Variables|Mesh|GetGravityMesh))
  (Rendering|Material|SetMaterial _mesh 0 (Variables|Mesh|GetMeshMaterial))
  (Transformation|SetWorldScale3D (Variables|Default|GetMesh) (Variables|Default|GetGravitionalForceScale))
  (Transformation|SetRelativeLocation _gravitycenterlocation (Variables|Default|GetGravityCenter) false false)
  (Variables|Default|SetGravityLocation (Transformation|GetWorldLocation _gravitycenterlocation)))